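; VR player pawn with floor-origin tracking, thumbstick teleport and two-handed physics object grabbing.
; While the right thumbstick is pressed, Tick traces from that controller and draws a debug cylinder as the target marker.
; Release teleports onto sufficiently flat surfaces, offset by the headset's horizontal position.
; Each trigger short-traces for physics bodies, disables simulation and attaches the actor to that hand, restoring physics on release.
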(event `Key|MotionController_Right_Thumbstick`
  (params (Key :type "Key Structure"))
  (:`Pressed`
    (set `self.ShowTeleportLocation` true))
  (:`Released`
    (set `self.ShowTeleportLocation` false)
    (if (`self.CanTeleport`)
      (`self.TeleportToLocation` (`self.TeleportLocation`)))))

(event `self.ReceiveTick`
  (params (DeltaSeconds :type "Float (single-precision)"))
  (bind _mc_right (`self.MC_Right`))
  (`self.TeleportGetLocation` (`SceneComponent.K2_GetComponentLocation` _mc_right) (`SceneComponent.GetForwardVector` _mc_right)))

(event `self.ReceiveBeginPlay`
  (`HeadMountedDisplayFunctionLibrary.SetTrackingOrigin` "Floor"))

(event `Key|MotionController_Left_Trigger`
  (params (Key :type "Key Structure"))
  ;[1 1 1] Pickup/dropping
  (:`Pressed`
    (if (not (`self.isHoldingObjectLeft`))
      (`self.PickUpObjectLeft`)))
  (:`Released`
    (`self.DropObjectLeft`)))

(event `Key|MotionController_Right_Trigger`
  (params (Key :type "Key Structure"))
  ;[1 1 1] Pickup/dropping
  (:`Pressed`
    (if (not (`self.IsHoldingObjectRight`))
      (`self.PickUpObjectRight`)))
  (:`Released`
    (`self.DropObjectRight`)))

(event `PickUpObjectLeft`
  (bind _hitcomponentleft (`self.HitComponentLeft`))
  (bind _mc_left (`self.MC_Left`))
  (bind _returnvalue (`SceneComponent.K2_GetComponentLocation` _mc_left))
  ;[1 1 1] Pickup/dropping
  ;;[1 1 1] Pickup left
  (bind (_outhit _returnvalue_2) (`KismetSystemLibrary.LineTraceSingleForObjects` _returnvalue (+ _returnvalue (* (`SceneComponent.GetForwardVector` _mc_left) 10)) (`|MakeArray` "ObjectTypeQuery4" :!type "EObjectTypeQuery Enum")))
  (if _returnvalue_2
    (bind (_bblockinghit _binitialoverlap _time _distance _location _impactpoint _normal _impactnormal _physmat _hitactor _hitcomponent) (`GameplayStatics.BreakHitResult` _outhit))
    (set `self.HitComponentLeft` _hitcomponent)
    (if (`SceneComponent.IsSimulatingPhysics` _hitcomponentleft "None")
      (bind _output_get (set `self.PickedUpActorLeft` _hitactor))
      (`PrimitiveComponent.SetSimulatePhysics` _hitcomponentleft false)
      (`SceneComponent.K2_AttachToComponent` (`Actor.RootComponent` _output_get) (`self.HeldObjectLocation_Left`) "None" "KeepWorld" "KeepWorld" "KeepWorld" true)
      (set `self.isHoldingObjectLeft` true))))

(event `DropObjectLeft`
  (bind _pickedupactorleft (`self.PickedUpActorLeft`))
  (bind _hitcomponentleft (`self.HitComponentLeft`))
  ;[1 1 1] Pickup/dropping
  ;;[1 1 1] Drop left
  (`/Engine/EditorBlueprintResources/StandardMacros.IsValid` _pickedupactorleft
    (:`Is Valid`
      (`self.K2_DetachFromActor` _pickedupactorleft "KeepWorld" "KeepWorld" "KeepWorld")
      (`/Engine/EditorBlueprintResources/StandardMacros.IsValid` _hitcomponentleft
        (:`Is Valid`
          (`PrimitiveComponent.SetSimulatePhysics` _hitcomponentleft true)
          (set `self.isHoldingObjectLeft` false)
          (set `self.HitComponentLeft` null)
          (set `self.PickedUpActorLeft` null))))))

(event `PickUpObjectRight`
  (bind _hitcomponentright (`self.HitComponentRight`))
  (bind _mc_right (`self.MC_Right`))
  (bind _returnvalue (`SceneComponent.K2_GetComponentLocation` _mc_right))
  ;[1 1 1] Pickup/dropping
  ;;[1 1 1] Pickup right
  (bind (_outhit _returnvalue_2) (`KismetSystemLibrary.LineTraceSingleForObjects` _returnvalue (+ _returnvalue (* (`SceneComponent.GetForwardVector` _mc_right) 10)) (`|MakeArray` "ObjectTypeQuery4" :!type "EObjectTypeQuery Enum")))
  (if _returnvalue_2
    (bind (_bblockinghit _binitialoverlap _time _distance _location _impactpoint _normal _impactnormal _physmat _hitactor _hitcomponent) (`GameplayStatics.BreakHitResult` _outhit))
    (set `self.HitComponentRight` _hitcomponent)
    (if (`SceneComponent.IsSimulatingPhysics` _hitcomponentright "None")
      (bind _output_get (set `self.PickedUpActorRight` _hitactor))
      (`PrimitiveComponent.SetSimulatePhysics` _hitcomponentright false)
      (`SceneComponent.K2_AttachToComponent` (`Actor.RootComponent` _output_get) (`self.HeldObjectLocation_Right`) "None" "KeepWorld" "KeepWorld" "KeepWorld" true)
      (set `self.IsHoldingObjectRight` true))))

(event `DropObjectRight`
  (bind _pickedupactorright (`self.PickedUpActorRight`))
  (bind _hitcomponentright (`self.HitComponentRight`))
  ;[1 1 1] Pickup/dropping
  ;;[1 1 1] Drop right
  (`/Engine/EditorBlueprintResources/StandardMacros.IsValid` _pickedupactorright
    (:`Is Valid`
      (`self.K2_DetachFromActor` _pickedupactorright "KeepWorld" "KeepWorld" "KeepWorld")
      (`/Engine/EditorBlueprintResources/StandardMacros.IsValid` _hitcomponentright
        (:`Is Valid`
          (`PrimitiveComponent.SetSimulatePhysics` _hitcomponentright true)
          (set `self.IsHoldingObjectRight` false)
          (set `self.HitComponentRight` null)
          (set `self.PickedUpActorRight` null))))))

(fn `TeleportGetLocation`
  (params (Position :type "Vector Structure") (ForwardVector :type "Vector Structure"))
  (if (`self.ShowTeleportLocation`)
    (bind _outhit (`KismetSystemLibrary.LineTraceSingle` Position (+ ForwardVector (* ForwardVector 10000.0)) "TraceTypeQuery1"))
    (bind (_bblockinghit _binitialoverlap _time _distance _location _impactpoint _normal) (`GameplayStatics.BreakHitResult` _outhit))
    (set `self.CanTeleport` (> (`KismetMathLibrary.Dot_VectorVector` _normal (0.0 0.0 1.0)) 0.75))
    (bind _output_get (set `self.TeleportLocation` _location))
    (`KismetSystemLibrary.DrawDebugCylinder` _output_get (+ _output_get (* _normal 20.0)) 50.0 32 (struct :`R` 0.162381 :`G` 0.849913 :`B` 1.0 :`A` 1.0))))

(fn `TeleportToLocation`
  (params (Location :type "Vector Structure"))
  (bind (_devicerotation _deviceposition) (`HeadMountedDisplayFunctionLibrary.GetOrientationAndPosition`))
  (`self.K2_SetActorLocation` (- Location (`KismetMathLibrary.MakeVector` (.x _deviceposition) (.y _deviceposition)))))

(fn `UserConstructionScript`)